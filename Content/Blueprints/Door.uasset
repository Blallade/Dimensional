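; Sliding double-door actor that opens and closes with sound, and resets when the player enters its trigger box.
; DoorAnimation drives a timeline that slides both panels in opposite directions up to DoorOpenedDistance, reversing it to close.
; On player overlap, it destroys every Portal actor in the level, closes the door, then calls DisableCollision and RestartButton on its assigned interruptor.
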(event OnComponentBeginOverlap(Box)
  (params (OverlappedComponent :type Primitive%20Component%20Object%20Reference) (OtherActor :type Actor%20Object%20Reference) (OtherComp :type Primitive%20Component%20Object%20Reference) (OtherBodyIndex :type Integer) (bFromSweep :type Boolean) (SweepResult :type Hit%20Result%20Structure%20%28by%20ref%29))
  (bind _asignedinterruptor (Variables|Default|GetAsignedInterruptor))
  (Utilities|Casting|CastToPlayer OtherActor)
  (CallFunction|ClearPortals)
  (CallFunction|DoorAnimation false)
  (Default|DisableCollision _asignedinterruptor false)
  (Default|RestartButton _asignedinterruptor))

(event Custom|DoorAnimation
  (params (Open :type Boolean))
  (if Open
    (Utilities|FlowControl|Sequence
      (:then_0
        (Audio|PlaySound2D 0 1.0 1.0 0.0 0 0))
      (:then_1
        (bind _alpha (Timeline|DoorAnim PlayFromStart)
          (:Update
            (Transformation|SetRelativeLocation (Variables|Default|GetDoorRight) (Math|Vector|MakeVector (Math|Float|Lerp 0.0 (Variables|Default|GetDoorOpenedDistance) _alpha) 0.0 0.0) false false)
            (Transformation|SetRelativeLocation (Variables|Default|GetDoorLeft) (Math|Vector|MakeVector (* (Math|Float|Lerp 0.0 (Variables|Default|GetDoorOpenedDistance) _alpha) -1.0) 0.0 0.0) false false)))))
    (else
      (Utilities|FlowControl|Sequence
        (:then_0
          (Timeline|DoorAnim Stop))
        (:then_1
          (Timeline|DoorAnim Reverse))
        (:then_2
          (Audio|PlaySound2D 0 1.0 1.0 0.0 0 0))))))

(fn ConstructionScript)

(fn ClearPortals
  (bind _outactors (Actor|GetAllActorsOfClass "/Game/Blueprints/Portal.Portal_C"))
  (for _array_element _outactors
    (Actor|DestroyActor _array_element))
  (return))