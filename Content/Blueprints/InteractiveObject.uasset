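; Interactive object actor that shows a "Press E" prompt when the player is inside its box and looking at it.
; Box overlap gates a Tick line trace from the first-person camera, with DoOnce nodes limiting prompt updates to changes.
; A hit matching this actor's class, not the specific instance, sets Player.InteractiveObject to self.
; Misses, hiding the prompt or toggling box collision clear that reference.
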(event OnComponentBeginOverlap(Box)
  (params (OverlappedComponent :type Primitive%20Component%20Object%20Reference) (OtherActor :type Actor%20Object%20Reference) (OtherComp :type Primitive%20Component%20Object%20Reference) (OtherBodyIndex :type Integer) (bFromSweep :type Boolean) (SweepResult :type Hit%20Result%20Structure%20%28by%20ref%29))
  (bind _asplayer (Utilities|Casting|CastToPlayer OtherActor))
  (Variables|Default|SetPlayer _asplayer)
  (Utilities|FlowControl|Gate true) ; enters at Open
)

(event OnComponentEndOverlap(Box)
  (params (OverlappedComponent :type Primitive%20Component%20Object%20Reference) (OtherActor :type Actor%20Object%20Reference) (OtherComp :type Primitive%20Component%20Object%20Reference) (OtherBodyIndex :type Integer))
  (Utilities|Casting|CastToPlayer OtherActor)
  (Utilities|FlowControl|Sequence
    (:then_0
      (Utilities|FlowControl|Gate true) ; enters at Close
    )
    (:then_1
      (Utilities|FlowControl|DoOnce false) ; enters at Reset
    )
    (:then_2
      (CallFunction|ShowInteractAdvice false))))

(event EventTick
  (params (DeltaSeconds :type Float%20%28single-precision%29))
  (Utilities|FlowControl|Gate true
    (:Exit
      (bind _buttondetected (CallFunction|CheckObjectAlongVector))
      (if _buttondetected
        (Utilities|FlowControl|Sequence
          (:then_0
            (Utilities|FlowControl|DoOnce false :!label _label
              (:Completed
                (CallFunction|ShowInteractAdvice true))))
          (:then_1
            (goto _label_2 Reset)))
        (else
          (Utilities|FlowControl|Sequence
            (:then_0
              (goto _label Reset))
            (:then_1
              (Utilities|FlowControl|DoOnce false :!label _label_2
                (:Completed
                  (CallFunction|ShowInteractAdvice false))))))))))

(fn ConstructionScript)

(fn CheckObjectAlongVector
  (bind _player (Variables|Default|GetPlayer))
  (bind _firstpersoncamera (Variables|/Game/Blueprints/Player.Player_C|GetFirstPersonCamera _player))
  (bind _returnvalue (Transformation|GetWorldLocation _firstpersoncamera))
  (bind _outhit (Collision|LineTraceForObjects _returnvalue (+ _returnvalue (* (Math|Vector|GetForwardVector _firstpersoncamera) (LocalVariables|GetSpawnDistance))) (Utilities|Array|MakeArray "ObjectTypeQuery2") false 0 "None" false))
  (if (== (Utilities|GetClass (.HitActor (Collision|BreakHitResult _outhit))) (Utilities|GetClass self))
    (Variables|/Game/Blueprints/Player.Player_C|SetInteractiveObject (Variables|Default|GetPlayer) self)
    (else
      (CallFunction|ClearReference)))
  (return (== (Utilities|GetClass (.HitActor (Collision|BreakHitResult _outhit))) (Utilities|GetClass self))))

(fn ShowInteractAdvice
  (params (Show? :type Boolean))
  (bind _foundwidgets (Widget|GetAllWidgetsOfClass "/Game/Blueprints/Widgets/UI.UI_C" true))
  (Default|PressEAdvice (Utilities|Array|Get(acopy) _foundwidgets) Show?)
  (if (not Show?)
    (CallFunction|ClearReference)
    (return)))

(fn DisableCollision
  (params (Disable? :type Boolean))
  (Collision|SetCollisionEnabled (Variables|Default|GetBox) (select Disable? "NoCollision" "QueryAndPhysics"))
  (CallFunction|ClearReference)
  (return))

(fn ClearReference
  (Variables|/Game/Blueprints/Player.Player_C|SetInteractiveObject (Variables|Default|GetPlayer) 0))