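; Interruptor is an interactable switch that opens its assigned door when the player uses it.
; On Interact it plays the button press animation and a 2D sound, then calls DoorAnimation on the assigned door if one is valid.
; It then disables its collision, while a separate RestartButton function resets the button animation.
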(event EventInteract
  (CallFunction|PressButton)
  (CallFunction|DisableCollision true))

(fn ConstructionScript
  (|CallParentFunction))

(fn PressButton
  (bind _asigneddoor (Variables|Default|GetAsignedDoor))
  (Components|Animation|PlayAnimation (Variables|Default|GetButton) "/Game/ThirdParty/Button/Animation/Anim_ButtonPressed.Anim_ButtonPressed" false)
  (Audio|PlaySound2D "/Game/Audio/ButtonPressed.ButtonPressed" 1.0 1.0 0.3 0 0)
  (Utilities|IsValid _asigneddoor
    (:Is%20Valid
      (Default|DoorAnimation _asigneddoor true))))

(fn RestartButton
  (Components|Animation|SetAnimation (Variables|Default|GetButton) 0))