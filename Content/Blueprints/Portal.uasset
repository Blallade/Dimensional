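; Linked A/B portal actor that shows a live view through its partner and teleports players across with relative view and velocity preserved.
; Tick resizes the render target to the scaled viewport and mirrors the player camera onto the partner's SceneCapture, with a distance-based near clip plane.
; Overlapping players switch to PortalPawn collision and teleport when their velocity-predicted position and last input point behind the portal plane.
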(event Collision|EventActorBeginOverlap
  (params (OtherActor :type Actor%20Object%20Reference))
  (Utilities|IsValid (Variables|Default|GetLinkedPortal)
    (:Is%20Valid
      (bind _asplayer (Utilities|Casting|CastToPlayer OtherActor))
      (bind _returnvalue (Utilities|Array|AddUnique (Variables|Default|GetPlayersInPortal) _asplayer))
      (if (!= _returnvalue -1)
        (Collision|SetCollisionProfileName (Variables|/Script/Engine.Character|GetCapsuleComponent _asplayer) "PortalPawn" true :!class /Script/Engine.PrimitiveComponent)))))

(event Collision|EventActorEndOverlap
  (params (OtherActor :type Actor%20Object%20Reference))
  (bind _asplayer (Utilities|Casting|CastToPlayer OtherActor))
  (Utilities|Array|RemoveItem (Variables|Default|GetPlayersInPortal) _asplayer)
  (Collision|SetCollisionProfileName (Variables|/Script/Engine.Character|GetCapsuleComponent _asplayer) "Pawn" true :!class /Script/Engine.PrimitiveComponent))

(event EventTick
  (params (DeltaSeconds :type Float%20%28single-precision%29))
  (bind _returnvalue (Game|GetPlayerCameraManager 0))
  (bind _returnvalue_2 (Viewport|GetViewportSize))
  (bind _portalquality (Variables|Default|GetPortalQuality))
  (bind _backfacingscene (Variables|Default|GetBackFacingScene))
  (bind _returnvalue_3 (Transformation|GetWorldTransform _backfacingscene))
  (bind _transformcomponent (Variables|/Script/Engine.PlayerCameraManager|GetTransformComponent _returnvalue))
  (bind _returnvalue_4 (Transformation|GetWorldTransform _transformcomponent))
  (bind _returnvalue_5 (Class|KismetMathLibrary|ConvertTransformtoRelative _returnvalue_3 _returnvalue_4))
  (Variables|Default|GetLinkedPortal
    (:then
      (Utilities|FlowControl|Sequence
        (:then_0
          (Class|PortalFunctionLibrary|ResizeRenderTarget (Variables|/Script/Engine.SceneCaptureComponent2D|GetTextureTarget (Variables|Default|GetSceneCapture)) (* (.x _returnvalue_2) _portalquality) (* (.y _returnvalue_2) _portalquality))
          (Transformation|SetRelativeLocationAndRotation (Variables|Portal_C|GetSceneCapture (Variables|Default|GetLinkedPortal)) (.location _returnvalue_5) (.rotation _returnvalue_5) false false)
          (Variables|/Script/Engine.SceneCaptureComponent2D|SetCustomNearClippingPlane (Variables|Portal_C|GetSceneCapture (Variables|Default|GetLinkedPortal)) (+ (Math|Vector|Distance(Vector) (Transformation|GetWorldLocation (Variables|/Script/Engine.PlayerCameraManager|GetTransformComponent (Game|GetPlayerCameraManager 0))) (Transformation|GetActorLocation)) 1.0)))
        (:then_1
          (for _array_element (Variables|Default|GetPlayersInPortal)
            (CallFunction|CheckifPlayerShouldTeleport _array_element)))))
    (:else)))

(fn ConstructionScript
  (Rendering|Material|SetMaterial (Variables|Default|GetPortalBorder) 0 (select (Variables|Default|GetPortalA) "/Game/Materials/MI_PortalBorderA.MI_PortalBorderA" "/Game/Materials/MI_PortalBorderB.MI_PortalBorderB"))
  (Variables|/Script/Engine.SceneCaptureComponent2D|SetTextureTarget (Variables|Default|GetSceneCapture) (select (Variables|Default|GetPortalA) "/Game/Materials/PortalRenderTargets/PortalRenderTargetA.PortalRenderTargetA" "/Game/Materials/PortalRenderTargets/PortalRenderTargetB.PortalRenderTargetB")))

(fn LinkPortals
  (params (Portal :type Portal%20Object%20Reference))
  (bind _output_get (Variables|Default|SetLinkedPortal Portal))
  (Utilities|IsValid _output_get
    (:Is%20Valid
      (Rendering|Material|SetMaterial (Variables|Default|GetPortal) 0 (select (Variables|Default|GetPortalA) "/Game/Materials/PortalRenderTargets/MI_PortalRenderTargetB.MI_PortalRenderTargetB" "/Game/Materials/PortalRenderTargets/MI_PortalRenderTargetA.MI_PortalRenderTargetA")))
    (:Is%20Not%20Valid
      (Rendering|Material|SetMaterial (Variables|Default|GetPortal) 0 "/Game/Materials/Colors/MI_DarkGrey.MI_DarkGrey"))))

(fn CheckifPlayerShouldTeleport
  (params (Player :type Player%20Object%20Reference))
  (if (and (<= (Math|Vector|DotProduct (Math|Vector|Normalize (- (+ (Transformation|GetActorLocation Player) (* (Transformation|GetVelocity Player) (Utilities|Time|GetWorldDeltaSeconds))) (Transformation|GetActorLocation))) (Transformation|GetActorForwardVector)) 0.0) (<= (Math|Vector|DotProduct (Math|Vector|Normalize (Class|Pawn|GetLastMovementInputVector Player)) (Transformation|GetActorForwardVector)) 0.0))
    (CallFunction|TeleportPlayer Player)))

(fn TeleportPlayer
  (params (Player :type Player%20Object%20Reference))
  (bind _backfacingscene (Variables|Default|GetBackFacingScene))
  (bind _linkedportal (Variables|Default|GetLinkedPortal))
  (bind _returnvalue (Transformation|GetWorldTransform _backfacingscene))
  (bind _returnvalue_2 (Transformation|GetActorTransform _linkedportal))
  (bind _firstpersoncamera (Variables|/Game/Blueprints/Player.Player_C|GetFirstPersonCamera Player))
  (bind _returnvalue_3 (Transformation|GetWorldTransform _firstpersoncamera))
  (bind _returnvalue_4 (Class|KismetMathLibrary|ConvertTransformtoRelative _returnvalue _returnvalue_3))
  (bind _returnvalue_5 (Math|Transform|ComposeTransforms _returnvalue_4 _returnvalue_2))
  (bind (_roll _pitch _yaw) (Math|Rotator|BreakRotator (.rotation _returnvalue_5)))
  (LocalVariables|SetRelativeVelocity (Math|Transform|InverseTransformDirection (Transformation|GetActorTransform Player) (Transformation|GetVelocity Player)))
  (Transformation|SetActorLocation Player (+ (* (Transformation|GetActorForwardVector (Variables|Default|GetLinkedPortal)) 16.0) (- (.location _returnvalue_5) (Variables|/Script/Engine.SceneComponent|GetRelativeLocation (Variables|/Game/Blueprints/Player.Player_C|GetFirstPersonCamera Player)))) false true)
  (Pawn|SetControlRotation (Pawn|GetController Player) (Math|Rotator|MakeRotator 0.0 _pitch _yaw))
  (Variables|/Script/Engine.MovementComponent|SetVelocity (Pawn|GetMovementComponent Player) (Math|Transform|TransformDirection (Math|Transform|MakeTransform (Transformation|GetActorLocation Player) (Pawn|GetControlRotation (Pawn|GetController Player) :!class /Script/Engine.Controller)) (LocalVariables|GetRelativeVelocity))))