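; PortalComponent places and links a pair of portals, A and B, on PortalWall surfaces.
; SpawnPortalAlongVector line traces along a direction and asks any hit PortalWall to add the chosen portal, nudged back toward the trace start.
; On success, SwapPortals destroys the old portal in that slot and stores the new one by reference, then both valid portals link to each other.
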(event EventBeginPlay)

(event EventTick
  (params (DeltaSeconds :type Float%20%28single-precision%29)))

(fn SpawnPortalAlongVector
  (params (StartLocation :type Vector) (Direction :type Vector) (PortalA :type Boolean))
  (bind _outhit (Collision|LineTraceForObjects StartLocation (+ StartLocation (* Direction (Variables|Default|GetMaxSpawnDistance))) (Utilities|Array|MakeArray "ObjectTypeQuery8" "ObjectTypeQuery1") false 0 "None"))
  (if (== (Utilities|GetClass (.HitActor (Collision|BreakHitResult _outhit))) "/Game/Blueprints/PortalWall.PortalWall_C")
    (bind _asportal_wall (Utilities|Casting|CastToPortalWall (.HitActor (Collision|BreakHitResult _outhit))))
    (bind _newportal (Default|TryAddPortal _asportal_wall (+ (.Location (Collision|BreakHitResult _outhit)) (* (Math|Vector|Normalize (- (.TraceStart (Collision|BreakHitResult _outhit)) (.TraceEnd (Collision|BreakHitResult _outhit)))) 1.0)) PortalA))
    (bind _output_get (Variables|Default|SetNewPortal _newportal))
    (Utilities|IsValid _output_get
      (:Is%20Valid
        (CallFunction|SwapPortals (select PortalA (Variables|Default|GetPortalA) (Variables|Default|GetPortalB)) (Variables|Default|GetNewPortal))
        (Utilities|FlowControl|Sequence
          (:then_0
            (bind _portala (Variables|Default|GetPortalA)
              (:then
                (Default|LinkPortals _portala (Variables|Default|GetPortalB)))
              (:else)))
          (:then_1
            (bind _portalb (Variables|Default|GetPortalB)
              (:then
                (Default|LinkPortals _portalb (Variables|Default|GetPortalA)))
              (:else))))))))

(fn SwapPortals
  (params (OldPortal :type Portal%20Object%20Reference%20%28by%20ref%29) (NewPortal :type Portal%20Object%20Reference))
  (Utilities|FlowControl|Sequence
    (:then_0
      (Utilities|IsValid OldPortal
        (:Is%20Valid
          (Actor|DestroyActor OldPortal))))
    (:then_1
      (|SetBy-RefVar OldPortal NewPortal))))