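; Project function library with a 2D axis-aligned rectangle overlap test.
; RectToRectCollision takes each rectangle as a center origin plus half-extents and compares their edges on X and Y.
; A sequence returns false at the first separating gap and true otherwise, so touching edges count as a collision.
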(fn RecttoRectCollision
  (params (Rect1Origin :type Vector%202D%20Structure) (Rect1Extents :type Vector%202D%20Structure) (Rect2Origin :type Vector%202D%20Structure) (Rect2Extents :type Vector%202D%20Structure))
  (Utilities|FlowControl|Sequence
    (:then_0
      (if (< (+ (.x Rect1Origin) (.x Rect1Extents)) (- (.x Rect2Origin) (.x Rect2Extents)))
        (return false)))
    (:then_1
      (if (> (- (.x Rect1Origin) (.x Rect1Extents)) (+ (.x Rect2Origin) (.x Rect2Extents)))
        (return false)))
    (:then_2
      (if (< (+ (.y Rect1Origin) (.y Rect1Extents)) (- (.y Rect2Origin) (.y Rect2Extents)))
        (return false)))
    (:then_3
      (if (> (- (.y Rect1Origin) (.y Rect1Extents)) (+ (.y Rect2Origin) (.y Rect2Extents)))
        (return false)))
    (:then_4
      (return true))))